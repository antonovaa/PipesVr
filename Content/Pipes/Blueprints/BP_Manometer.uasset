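; BP_Manometer is a pressure gauge Blueprint that shows a pressure value with a rotating arrow.
; It extends the parent's SetPressure, mapping pressure from its minimum–maximum range to a clamped angle range and applying it as the arrow's relative roll.
; The construction script runs the parent's, then rolls the pipe mesh (SMTrubka) by a configurable PipeRotation.
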(event `self.SetPressure`
  (params (Pressure :type "Float (single-precision)"))
  (`parent.SetPressure` Pressure)
  (`SceneComponent.K2_SetRelativeRotation` (`self.SM_ManometerArrow`) (`KismetMathLibrary.MakeRotator` (`KismetMathLibrary.MapRangeClamped` (`self.Pressure`) (`self.Mininmum`) (`self.Maximum`) (`self.MinAngle`) (`self.MaxAngle`))) false false)
  (if true
    _))

(fn `UserConstructionScript`
  (`parent.UserConstructionScript`)
  (`SceneComponent.K2_SetRelativeRotation` (`self.SM_Trubka`) (`KismetMathLibrary.MakeRotator` (`self.PipeRotation`)) false false))