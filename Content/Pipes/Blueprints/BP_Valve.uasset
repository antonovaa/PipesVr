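; Grabbable valve for a pipe repair level that turns with the grabbing sphere, with steam effects and a repair widget.
; While the pawn overlaps it, Tick accumulates a clamped angle from the target's direction changes around the actor's up axis.
; UpdatePosition turns and raises the handle like a screw and returns openness to PC_Pipes for checking.
; Switchers 1 and 2 restart the level as wrong choices; sounds differ at end stops.
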(event `StopEffects`
  (`ActorComponent.Deactivate` (`self.Wave`))
  (`ActorComponent.Deactivate` (`self.steam`)))

(event `startEffects`
  (params (Count :type Integer))
  (`ActorComponent.Activate` (`self.Wave`) false)
  (`ActorComponent.Activate` (`self.steam`) false)
  (bind _asrepair_widget (cast `/Game/Pipes/Menu/RepairWidget` (`WidgetComponent.GetUserWidgetObject` (`self.RepairWidget`))))
  (set `/Game/Pipes/Menu/RepairWidget.Count` Count _asrepair_widget))

(event `self.ReceiveBeginPlay`
  ;[1 1 1] init
  (bind _aspc_pipes (cast `/Game/Pipes/Blueprints/PC_Pipes` (`GameplayStatics.GetPlayerController` 0)))
  (set `self.PC_Pipes` _aspc_pipes)
  (bind _asrepair_widget (cast `/Game/Pipes/Menu/RepairWidget` (`WidgetComponent.GetUserWidgetObject` (`self.RepairWidget`))))
  (set `/Game/Pipes/Menu/RepairWidget.ValveType` (`self.Name`) _asrepair_widget)
  (`SceneComponent.SetVisibility` (`self.RepairWidget`) true false))

(event `Grab_1`
  (params (TargetSphere :type "SphereComponent Object Reference"))
  ;[1 1 1] trigger on/off
  (set `self.setcheck` true)
  (bind _output_get (set `self.Target` TargetSphere))
  (set `self.InitLocation` (`KismetMathLibrary.Normal` (`KismetMathLibrary.ProjectVectorOnToPlane` (- (`SceneComponent.K2_GetComponentLocation` _output_get) (`SceneComponent.K2_GetComponentLocation` (`self.Mesh`))) (`self.GetActorUpVector`))))
  (`ActorComponent.Activate` (`self.Audio`) false))

(event `Drop_1`
  ;[1 1 1] trigger on/off
  (set `self.setcheck` false)
  (set `self.Target` null)
  (`self.ResetSound`)
  (`ActorComponent.Deactivate` (`self.Audio`)))

(event `self.ReceiveTick`
  (params (DeltaSeconds :type "Float (single-precision)"))
  (bind _audio (`self.Audio`))
  (bind _switchernumber (`self.SwitcherNumber`))
  (bind _open (`self.Open`))
  (bind _pc_pipes (`self.PC_Pipes`))
  ;[1 1 1] calc open
  (if (not (`self.isBroke`))
    (`/Engine/EditorBlueprintResources/StandardMacros.Gate` true :!label _label
      (:`Exit`
        (if (`self.setcheck`)
          (bind _target (`self.Target`)
            (:`then`
              (bind _returnvalue (`KismetMathLibrary.Normal` (- (`SceneComponent.K2_GetComponentLocation` _target) (`SceneComponent.K2_GetComponentLocation` (`self.Mesh`)))))
              (set `self.Angle` (`KismetMathLibrary.FClamp` (- (`self.Angle`) (`self.Determinant` _returnvalue (`self.InitLocation`) (`self.GetActorUpVector`))) 0.0 (`self.MaxAngle`)))
              (set `self.InitLocation` _returnvalue)
              (bind _open_2 (`self.UpdatePosition`))
              (if (or (== _switchernumber 1) (== _switchernumber 2))
                (`/Game/Pipes/Blueprints/PC_Pipes.RepeatLevel` _pc_pipes "Неверно. Попробуйте еще!")
                (else
                  (`/Game/Pipes/Blueprints/PC_Pipes.CheckRight` _pc_pipes (`self.SwitcherNumber`) _open_2)))
              (if (or (== _open 0.0) (== _open 1.0))
                (`/Engine/EditorBlueprintResources/StandardMacros.DoOnce` false :!label _label_2
                  (:`Completed`
                    (`AudioComponent.SetSound` _audio "/Game/Pipes/Sounds/valve_close.valve_close")
                    (`KismetSystemLibrary.Delay` 5.1)
                    (`self.ResetSound`)))
                (else
                  (`/Engine/EditorBlueprintResources/StandardMacros.DoOnce` false :!label _label_3
                    (:`Completed`
                      (`AudioComponent.SetSound` _audio "/Game/Pipes/Sounds/valve.valve")
                      (`KismetSystemLibrary.Delay` 0.4)
                      (`self.ResetSound`))))))
            (:`else`)))))))

(event `openGate`
  ;[1 1 1] calc open
  (goto _label :!via `Open`))

(event `ResetSound`
  ;[1 1 1] calc open
  (`|ExecutionSequence`
    (:`then_0`
      (goto _label_2 :!via `Reset`))
    (:`then_1`
      (goto _label_3 :!via `Reset`))))

(event `CloseGate`
  ;[1 1 1] calc open
  (goto _label :!via `Close`))

(event `self.Mesh.OnComponentBeginOverlap`
  (params (OverlappedComponent :type "PrimitiveComponent Object Reference") (OtherActor :type "Actor Object Reference") (OtherComp :type "PrimitiveComponent Object Reference") (OtherBodyIndex :type Integer) (bFromSweep :type Boolean) (SweepResult :type "HitResult Structure (by ref)"))
  ;[1 1 1] overlap with controller
  (cast `/Game/Pipes/Blueprints/Pawn_Pipes` OtherActor)
  (`PrimitiveComponent.SetRenderCustomDepth` (`self.Mesh`) true)
  (`self.openGate`))

(event `self.Mesh.OnComponentEndOverlap`
  (params (OverlappedComponent :type "PrimitiveComponent Object Reference") (OtherActor :type "Actor Object Reference") (OtherComp :type "PrimitiveComponent Object Reference") (OtherBodyIndex :type Integer))
  ;[1 1 1] overlap with controller
  (cast `/Game/Pipes/Blueprints/Pawn_Pipes` OtherActor)
  (`PrimitiveComponent.SetRenderCustomDepth` (`self.Mesh`) false)
  (`self.CloseGate`)
  (`ActorComponent.Deactivate` (`self.Audio`)))

(fn `UpdatePosition`
  (returns (Open :type "Float (double-precision)"))
  (set `self.Height` (* (/ (`self.Angle`) 360.0) (`self.Stroke`)))
  (`SceneComponent.K2_SetRelativeLocationAndRotation` (`self.Mesh`) (`KismetMathLibrary.MakeVector` 0.0 0.0 (`self.Height`)) (`KismetMathLibrary.MakeRotator` 0.0 0.0 (`self.Angle`)) false false)
  (bind _output_get (set `self.Open` (`KismetMathLibrary.MapRangeClamped` (`self.Angle`) 0.0 (`self.MaxAngle`) 0.0 1.0)))
  (return _output_get))

(fn `UserConstructionScript`
  (bind _repairwidget (`self.RepairWidget`))
  (bind _isvisible (`self.isVisible`))
  (bind _wave (`self.Wave`))
  (`parent.UserConstructionScript`)
  (`self.UpdatePosition`)
  (`SceneComponent.K2_SetWorldRotation` _repairwidget (struct :`Yaw` 180.0) false false)
  (`SceneComponent.SetVisibility` _repairwidget _isvisible false)
  (`SceneComponent.K2_SetRelativeLocation` _repairwidget (`self.WidgetLocation`) false false)
  (`ActorComponent.SetAutoActivate` (`self.P_Steam_Lit`) _isvisible)
  (`SceneComponent.K2_SetRelativeRotation` _wave (`self.WaveRotation`) false false)
  (`ParticleSystemComponent.SetVectorParameter` _wave "Fog Intensity" (`self.EmmiterParams`))
  (`ActorComponent.SetAutoActivate` _wave _isvisible))