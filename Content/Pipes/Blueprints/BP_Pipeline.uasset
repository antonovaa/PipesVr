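; BP_Pipeline simulates pressure through a fixed network of pipe knots and valves and drives the BP_Manometer gauges in the level.
; Each tick it resets knot pressures with two full-pressure sources, then multiplies pressure by valve openness along two parallel lines.
; A cross-link valve shares pressure between the middle knots, keeping the higher value.
; Manometers, gathered on BeginPlay, then receive the pressure of their assigned knot.
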(event `self.ReceiveBeginPlay`
  (bind _outactors (`GameplayStatics.GetAllActorsOfClass` "/Game/Pipes/Blueprints/BP_Manometer.BP_Manometer_C"))
  (set `self.Manometers` _outactors))

(event `self.ReceiveTick`
  (params (DeltaSeconds :type "Float (single-precision)"))
  (bind (_output_type _output_pressure) (break `/Game/Pipes/Blueprints/S_Knot` (`|GetArrayItem` (`self.Knots`) 1)))
  (bind (_output_type_2 _output_pressure_2) (break `/Game/Pipes/Blueprints/S_Knot` (`|GetArrayItem` (`self.Knots`))))
  (bind (_output_type_3 _output_pressure_3) (break `/Game/Pipes/Blueprints/S_Knot` (`|GetArrayItem` (`self.Knots`) 4)))
  (bind (_output_type_4 _output_pressure_4) (break `/Game/Pipes/Blueprints/S_Knot` (`|GetArrayItem` (`self.Knots`) 3)))
  (bind (_output_type_5 _output_pressure_5) (break `/Game/Pipes/Blueprints/S_Knot` (`|GetArrayItem` (`self.Knots`) 1)))
  (bind (_output_type_6 _output_pressure_6) (break `/Game/Pipes/Blueprints/S_Knot` (`|GetArrayItem` (`self.Knots`) 4)))
  (bind (_output_type_7 _output_pressure_7) (break `/Game/Pipes/Blueprints/S_Knot` (`|GetArrayItem` (`self.Knots`) 4)))
  (bind (_output_type_8 _output_pressure_8) (break `/Game/Pipes/Blueprints/S_Knot` (`|GetArrayItem` (`self.Knots`) 1)))
  (for (_array_element _array_index) (`self.Knots`)
    (bind _structout (setmembers `/Game/Pipes/Blueprints/S_Knot` :`StructRef` _array_element :`Pressure` (`KismetMathLibrary.SelectFloat` 1.0 0.0 (or (== _array_index 0) (== _array_index 3)))))
    (`KismetArrayLibrary.Array_Set` (`self.Knots`) _array_index _structout))
  (setmembers `/Game/Pipes/Blueprints/S_Knot` :`StructRef` (`|GetArrayItem` (`self.Knots`) 1) :`Pressure` (* _output_pressure_2 (`/Game/Pipes/Blueprints/BP_Section.Open` (`|GetArrayItem` (`self.Valves`)))))
  (setmembers `/Game/Pipes/Blueprints/S_Knot` :`StructRef` (`|GetArrayItem` (`self.Knots`) 4) :`Pressure` (* _output_pressure_4 (`/Game/Pipes/Blueprints/BP_Section.Open` (`|GetArrayItem` (`self.Valves`) 3))))
  (setmembers `/Game/Pipes/Blueprints/S_Knot` :`StructRef` (`|GetArrayItem` (`self.Knots`) 1) :`Pressure` (`KismetMathLibrary.FMax` _output_pressure_8 (* _output_pressure_3 (`/Game/Pipes/Blueprints/BP_Section.Open` (`|GetArrayItem` (`self.Valves`) 2)))))
  (setmembers `/Game/Pipes/Blueprints/S_Knot` :`StructRef` (`|GetArrayItem` (`self.Knots`) 4) :`Pressure` (`KismetMathLibrary.FMax` _output_pressure_6 (* _output_pressure (`/Game/Pipes/Blueprints/BP_Section.Open` (`|GetArrayItem` (`self.Valves`) 2)))))
  (setmembers `/Game/Pipes/Blueprints/S_Knot` :`StructRef` (`|GetArrayItem` (`self.Knots`) 2) :`Pressure` (* _output_pressure_5 (`/Game/Pipes/Blueprints/BP_Section.Open` (`|GetArrayItem` (`self.Valves`) 1))))
  (setmembers `/Game/Pipes/Blueprints/S_Knot` :`StructRef` (`|GetArrayItem` (`self.Knots`) 5) :`Pressure` (* _output_pressure_7 (`/Game/Pipes/Blueprints/BP_Section.Open` (`|GetArrayItem` (`self.Valves`) 4))))
  (for _array_element_2 (`self.Manometers`)
    (bind (_output_type_9 _output_pressure_9) (break `/Game/Pipes/Blueprints/S_Knot` (`|GetArrayItem` (`self.Knots`) (`/Game/Pipes/Blueprints/BP_Manometer.OnKnot` _array_element_2))))
    (`/Game/Pipes/Blueprints/BP_Section.SetPressure` _array_element_2 _output_pressure_9)))

(fn `UserConstructionScript`)