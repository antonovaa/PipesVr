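; Player pawn for the pipes game, using a motion controller with an optional mouse-and-keyboard mode for look and movement.
; Use grabs and releases an overlapping BP_Valve, or confirms the active menu choice.
; The main menu widget selects difficulty on GI_Pipes and loads the map, or quits.
; In menu states, Tick line-traces along the controller to cache the valve's RepairWidget, whose checked state lets Use end repair through PC_Pipes.
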(event `stopMuneWidget`
  (bind _widget (`self.Widget`))
  ;[1 1 1] start on game map
  (`SceneComponent.SetVisibility` _widget false false)
  (`PrimitiveComponent.SetCollisionEnabled` _widget "NoCollision")
  (set `self.IsInMenu` false)
  (set `self.IsInRepairMenu` false))

(event `self.ReceiveBeginPlay`
  ;[1 1 1] init
  (if (`self.MouseInput`)
    (`SceneComponent.K2_AttachToComponent` (`self.StaticMesh`) (`self.Camera`) "None" "KeepRelative" "KeepRelative" "KeepRelative" true)
    (`SceneComponent.K2_SetRelativeLocation` (`self.StaticMesh`) (100.0 0.0 -50.0) false false)
    (set `CameraComponent.bUsePawnControlRotation` true (`self.Camera`))))

(event `InputAction|Use`
  (params (Key :type "Key Structure"))
  (bind _isinmenu (`self.IsInMenu`))
  ;[1 1 1] Trigger On/Off
  (:`Pressed`
    (if _isinmenu
      (`self.getNumberButton`)
      (elif (`self.IsInRepairMenu`)
        (`self.getIsInChecked`)
        (else
          (for _array_element (`PrimitiveComponent.GetOverlappingActors` (`self.Sphere`) "/Game/Pipes/Blueprints/BP_Valve.BP_Valve_C")
            (bind _asbp_valve (cast `/Game/Pipes/Blueprints/BP_Valve` _array_element))
            (bind _output_get (set `self.UsingActor` _asbp_valve))
            (`/Game/Pipes/Blueprints/BP_Valve.Grab_1` _output_get (`self.Sphere`))
            (break))))))
  (:`Released`
    (if _isinmenu
      _
      (elif (not (`self.IsInRepairMenu`))
        (bind _usingactor (`self.UsingActor`)
          (:`then`
            (`/Game/Pipes/Blueprints/BP_Valve.Drop_1` _usingactor)
            (set `self.UsingActor` null))
          (:`else`))))))

(event `getNumberButton`
  (bind _returnvalue (`GameplayStatics.GetGameInstance`))
  ;[1 1 1] open Level or exit
  (bind _asmenu_widget (cast `/Game/Pipes/Menu/MenuWidget` (`WidgetComponent.GetUserWidgetObject` (`self.Widget`))))
  (bind _output_get (set `self.numberKey` (`/Game/Pipes/Menu/MenuWidget.NumberButton` _asmenu_widget)))
  (if (== _output_get 1)
    (`ActorComponent.Activate` (`self.PUSH_THE_BUTTON`) false)
    (bind _asgi_pipes (cast `/Game/Pipes/Blueprints/GI_Pipes` _returnvalue))
    (set `/Game/Pipes/Blueprints/GI_Pipes.isHard` true _asgi_pipes)
    (`GameplayStatics.OpenLevel` "Map" :!label _label)
    (elif (== _output_get 0)
      (`ActorComponent.Activate` (`self.PUSH_THE_BUTTON`) false)
      (bind _asgi_pipes_2 (cast `/Game/Pipes/Blueprints/GI_Pipes` _returnvalue))
      (set `/Game/Pipes/Blueprints/GI_Pipes.isHard` false _asgi_pipes_2)
      (goto _label)
      (elif (== _output_get 2)
        (`ActorComponent.Activate` (`self.PUSH_THE_BUTTON`) false)
        (`KismetSystemLibrary.QuitGame` null "Quit")))))

(event `getIsInChecked`
  (bind _repairwidget (`self.RepairWidget`))
  (bind _push_the_button (`self.PUSH_THE_BUTTON`))
  ;[1 1 1] repairing
  (`/Engine/EditorBlueprintResources/StandardMacros.IsValid` _repairwidget
    (:`Is Valid`
      (if (`/Game/Pipes/Menu/RepairWidget.isInChecked` _repairwidget)
        (`ActorComponent.Activate` _push_the_button false)
        (`AudioComponent.Play` _push_the_button 0.0)
        (bind _aspc_pipes (cast `/Game/Pipes/Blueprints/PC_Pipes` (`self.GetController`)))
        (`/Game/Pipes/Blueprints/PC_Pipes.EndRepair` _aspc_pipes)))))

(event `PlayHoveredSound`
  (`ActorComponent.Activate` (`self.navedenie_na_knopku`) false))

(event `self.ReceiveTick`
  (params (DeltaSeconds :type "Float (single-precision)"))
  (bind _camera (`self.Camera`))
  (bind _returnvalue (`SceneComponent.K2_GetComponentLocation` (`self.StaticMesh`)))
  ;[1 1 1] linetrace for menu
  (if (or (`self.IsInMenu`) (`self.IsInRepairMenu`))
    (bind _outhit (`KismetSystemLibrary.LineTraceSingleForObjects` :`Start` _returnvalue :`End` (+ _returnvalue (* (`SceneComponent.GetForwardVector` (`self.MotionController`)) 10000.0)) :`ObjectTypes` (`|MakeArray` "ObjectTypeQuery7" :!type "EObjectTypeQuery Enum") :`DrawDebugType` "ForOneFrame" :`bIgnoreSelf` false))
    (bind (_bblockinghit _binitialoverlap _time _distance _location _impactpoint _normal _impactnormal _physmat _hitactor _hitcomponent) (`GameplayStatics.BreakHitResult` _outhit))
    (bind _asbp_valve (cast `/Game/Pipes/Blueprints/BP_Valve` _hitactor))
    (bind _asrepair_widget (cast `/Game/Pipes/Menu/RepairWidget` (`WidgetComponent.GetUserWidgetObject` (`/Game/Pipes/Blueprints/BP_Valve.RepairWidget` _asbp_valve))))
    (set `self.RepairWidget` _asrepair_widget)
    (`KismetSystemLibrary.PrintString` (`KismetSystemLibrary.GetDisplayName` _hitcomponent) true true (struct :`G` 0.66 :`B` 1.0 :`A` 1.0) 0.0)
    (else
      (`|ExecutionSequence`
        (:`then_1`
          (if (`self.MouseInput`)
            (`self.AddControllerPitchInput` (`self.GetInputAxisValue`))
            (`self.AddControllerYawInput` (`self.GetInputAxisValue`))
            (`self.K2_AddActorWorldOffset` (* (`KismetMathLibrary.Normal` (+ (* (`SceneComponent.GetRightVector` _camera) (`self.GetInputAxisValue`)) (* (`SceneComponent.GetForwardVector` _camera) (`self.GetInputAxisValue`)))) (* 200.0 (`GameplayStatics.GetWorldDeltaSeconds`))))))))))

(fn `UserConstructionScript`)