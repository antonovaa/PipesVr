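; GS_Pipes, likely the game state for a pipe and valve puzzle, is a mostly stubbed Blueprint that tracks valve readiness.
; CheckReadyOpen flags valve 4 as ready when its open amount reaches 0.9; its branches for valves 3 and 5 do nothing.
; StartNewGame is empty, and a disconnected fragment that searches map keys and adds entries never runs.
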(event `StartNewGame`)

(event `CheckReadyOpen`
  (params (Number :type Integer) (Open :type "Float (double-precision)"))
  (if (== Number 4)
    (set `self.readyValve4` (>= Open 0.9))
    (elif (== Number 5)
      _
      (elif (== Number 3)
        _))))

(fn `UserConstructionScript`)