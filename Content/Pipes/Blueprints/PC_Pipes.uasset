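; Player controller for the pipe puzzle that checks valve order: open 4, open 5, then close 3.
; An out-of-order valve triggers RepeatLevel, which shows an error, fades the camera and resets all valves.
; Success shows a victory message and loads StartMap, except on hard mode.
; There, a counter breaks valves 3, 4 and 5 on successive successes, and EndRepair restores each and restarts the puzzle before the final win.
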(event `self.ReceiveBeginPlay`
  ;[1 1 1] Init
  (`KismetSystemLibrary.Delay` 1.0)
  (bind _aspawn_pipes (cast `/Game/Pipes/Blueprints/Pawn_Pipes` (`self.K2_GetPawn`)))
  (set `self.Pawn_Pipes` _aspawn_pipes))

(event `RepeatLevel`
  (params (Text :type String))
  (bind _bp_widgetfinal (`self.BP_WidgetFinal`))
  (bind _returnvalue (`WidgetComponent.GetUserWidgetObject` (`/Game/Pipes/Blueprints/BP_WidgerTitle.Final` _bp_widgetfinal)))
  ;[1 1 1] Error play game
  (`PlayerCameraManager.StartCameraFade` :`self` (`GameplayStatics.GetPlayerCameraManager` 0) :`ToAlpha` 1.0 :`Duration` 3.0 :`bHoldWhenFinished` true)
  (`AudioComponent.Play` (`/Game/Pipes/Blueprints/BP_WidgerTitle.info_message` _bp_widgetfinal) 0.0)
  (bind _asfinal (cast `/Game/Pipes/Menu/Final` _returnvalue))
  (`/Game/Pipes/Menu/Final.set color` _asfinal false)
  (set `/Game/Pipes/Menu/Final.Text` Text _asfinal)
  (`Widget.SetVisibility` _returnvalue "Visible")
  (`KismetSystemLibrary.Delay` 3.0)
  (bind _outactors (`GameplayStatics.GetAllActorsOfClass` "/Game/Pipes/Blueprints/BP_Valve.BP_Valve_C"))
  (for _array_element _outactors
    (bind _asbp_valve (cast `/Game/Pipes/Blueprints/BP_Valve` _array_element))
    (bind _switchernumber (`/Game/Pipes/Blueprints/BP_Valve.SwitcherNumber` _asbp_valve))
    (if (or (== _switchernumber 1) (== _switchernumber 3))
      (set `/Game/Pipes/Blueprints/BP_Valve.Angle` 720.0 _asbp_valve)
      (`/Game/Pipes/Blueprints/BP_Valve.UpdatePosition` _asbp_valve)
      (else
        (set `/Game/Pipes/Blueprints/BP_Valve.Angle` 0.0 _asbp_valve)
        (`/Game/Pipes/Blueprints/BP_Valve.UpdatePosition` _asbp_valve))))
  (`Widget.SetVisibility` _returnvalue "Hidden")
  (`PlayerCameraManager.StartCameraFade` :`self` (`GameplayStatics.GetPlayerCameraManager` 0) :`FromAlpha` 1.0 :`Duration` 1.0)
  ;;[1 1 1] true -- как надо
  (set `self.Valve4` false)
  (set `self.Valve5` false)
  (set `self.Valve3` false))

(event `CheckRight`
  (params (Number :type Integer) (Open :type "Float (double-precision)"))
  ;[1 1 1] Check
  (if (== Number 4)
    (if (>= Open 0.9)
      (set `self.Valve4` true)
      (else
        (set `self.Valve4` false)))
    (elif (and (== Number 5) (`self.Valve4`))
      (if (>= Open 0.9)
        (set `self.Valve5` true)
        (else
          (set `self.Valve5` false)))
      (elif (and (== Number 3) (`self.Valve5`))
        (if (<= Open 0.1)
          (`self.PlayTonext`))
        (else
          (`self.RepeatLevel` "Неверно. Попробуйте еще!"))))))

(event `Repair`
  (bind _bp_widgetfinal (`self.BP_WidgetFinal`))
  (bind _returnvalue (`WidgetComponent.GetUserWidgetObject` (`/Game/Pipes/Blueprints/BP_WidgerTitle.Final` _bp_widgetfinal)))
  ;[1 1 1] comment
  (`AudioComponent.Play` (`/Game/Pipes/Blueprints/BP_WidgerTitle.info_message` _bp_widgetfinal) 0.0)
  (bind _asfinal (cast `/Game/Pipes/Menu/Final` _returnvalue))
  (set `/Game/Pipes/Menu/Final.Text` "Нужен ремонт!" _asfinal)
  (`/Game/Pipes/Menu/Final.set color` _asfinal false)
  (`Widget.SetVisibility` _returnvalue "Visible")
  (`KismetSystemLibrary.Delay` 5.0)
  (`Widget.SetVisibility` _returnvalue "Hidden")
  (`self.ResetOnce`))

(event `PlayToNext`
  (bind _bp_valve3 (`self.BP_Valve3`))
  (bind _bp_valve4 (`self.BP_Valve4`))
  (bind _bp_valve5 (`self.BP_Valve5`))
  ;[1 1 1] Success complite level
  (bind _asgi_pipes (cast `/Game/Pipes/Blueprints/GI_Pipes` (`GameplayStatics.GetGameInstance`)))
  (`/Engine/EditorBlueprintResources/StandardMacros.DoOnce` false :!label _label
    (:`Completed`
      (if (`/Game/Pipes/Blueprints/GI_Pipes.isHard` _asgi_pipes)
        (switch `int` (`self.count`)
          (:`Default`
            (`self.GoToMenu`))
          (:`0`
            (`Widget.SetVisibility` (`WidgetComponent.GetUserWidgetObject` (`/Game/Pipes/Blueprints/BP_Valve.RepairWidget` _bp_valve3)) "Visible")
            (`MeshComponent.SetVectorParameterValueOnMaterials` (`/Game/Pipes/Blueprints/BP_Valve.Mesh` _bp_valve3) "ColorRed" (256.0 0.0 0.0))
            (set `/Game/Pipes/Blueprints/BP_Valve.isBroke` true _bp_valve3)
            (`/Game/Pipes/Blueprints/BP_Valve.startEffects` _bp_valve3 5)
            (`self.Repair` :!label _label_2)
            (set `/Game/Pipes/Blueprints/Pawn_Pipes.IsInRepairMenu` true (`self.Pawn_Pipes`)))
          (:`1`
            (`Widget.SetVisibility` (`WidgetComponent.GetUserWidgetObject` (`/Game/Pipes/Blueprints/BP_Valve.RepairWidget` _bp_valve4)) "Visible")
            (`MeshComponent.SetVectorParameterValueOnMaterials` (`/Game/Pipes/Blueprints/BP_Valve.Mesh` _bp_valve4) "ColorRed" (256.0 0.0 0.0))
            (set `/Game/Pipes/Blueprints/BP_Valve.isBroke` true _bp_valve4)
            (`/Game/Pipes/Blueprints/BP_Valve.startEffects` _bp_valve4 4)
            (goto _label_2))
          (:`2`
            (`Widget.SetVisibility` (`WidgetComponent.GetUserWidgetObject` (`/Game/Pipes/Blueprints/BP_Valve.RepairWidget` _bp_valve5)) "Visible")
            (`MeshComponent.SetVectorParameterValueOnMaterials` (`/Game/Pipes/Blueprints/BP_Valve.Mesh` _bp_valve5) "ColorRed" (256.0 0.0 0.0))
            (set `/Game/Pipes/Blueprints/BP_Valve.isBroke` true _bp_valve5)
            (`/Game/Pipes/Blueprints/BP_Valve.startEffects` _bp_valve5 3)
            (goto _label_2)))
        (else
          (`self.GoToMenu`))))))

(event `ResetOnce`
  ;[1 1 1] Success complite level
  (goto _label :!via `Reset`))

(event `EndRepair`
  (bind _bp_valve3 (`self.BP_Valve3`))
  (bind _bp_valve4 (`self.BP_Valve4`))
  (bind _bp_valve5 (`self.BP_Valve5`))
  (bind _repairwidget (`/Game/Pipes/Blueprints/BP_Valve.RepairWidget` _bp_valve5))
  (bind _repairwidget_2 (`/Game/Pipes/Blueprints/BP_Valve.RepairWidget` _bp_valve3))
  (bind _repairwidget_3 (`/Game/Pipes/Blueprints/BP_Valve.RepairWidget` _bp_valve4))
  ;[1 1 1] after repair
  (switch `int` (`self.count`)
    (:`Default`
      (`self.GoToMenu`))
    (:`0`
      (`Widget.SetVisibility` (`WidgetComponent.GetUserWidgetObject` _repairwidget_2) "Hidden")
      (`PrimitiveComponent.SetCollisionEnabled` _repairwidget_2 "NoCollision")
      (`MeshComponent.SetVectorParameterValueOnMaterials` (`/Game/Pipes/Blueprints/BP_Valve.Mesh` _bp_valve3) "ColorRed" (0.0 0.0 2.0))
      (set `/Game/Pipes/Blueprints/BP_Valve.isBroke` false _bp_valve3)
      (`/Game/Pipes/Blueprints/BP_Valve.StopEffects` _bp_valve3)
      (set `/Game/Pipes/Blueprints/Pawn_Pipes.IsInRepairMenu` false (`self.Pawn_Pipes`) :!label _label_3)
      (`/Engine/EditorBlueprintResources/StandardMacros.IncrementInt` (`self.count`)
        (:`  `
          (`self.RepeatLevel` ""))))
    (:`1`
      (`Widget.SetVisibility` (`WidgetComponent.GetUserWidgetObject` _repairwidget_3) "Hidden")
      (`PrimitiveComponent.SetCollisionEnabled` _repairwidget_3 "NoCollision")
      (`MeshComponent.SetVectorParameterValueOnMaterials` (`/Game/Pipes/Blueprints/BP_Valve.Mesh` _bp_valve4) "ColorRed" (0.0 0.0 2.0))
      (set `/Game/Pipes/Blueprints/BP_Valve.isBroke` false _bp_valve4)
      (`/Game/Pipes/Blueprints/BP_Valve.StopEffects` _bp_valve4)
      (goto _label_3))
    (:`2`
      (`Widget.SetVisibility` (`WidgetComponent.GetUserWidgetObject` _repairwidget) "Hidden")
      (`PrimitiveComponent.SetCollisionEnabled` _repairwidget "NoCollision")
      (`MeshComponent.SetVectorParameterValueOnMaterials` (`/Game/Pipes/Blueprints/BP_Valve.Mesh` _bp_valve5) "ColorRed" (0.0 0.0 2.0))
      (set `/Game/Pipes/Blueprints/BP_Valve.isBroke` false _bp_valve5)
      (`/Game/Pipes/Blueprints/BP_Valve.StopEffects` _bp_valve5)
      (goto _label_3))))

(event `GoToMenu`
  (bind _bp_widgetfinal (`self.BP_WidgetFinal`))
  (bind _returnvalue (`WidgetComponent.GetUserWidgetObject` (`/Game/Pipes/Blueprints/BP_WidgerTitle.Final` _bp_widgetfinal)))
  ;[1 1 1] go to new game
  (`PlayerCameraManager.StartCameraFade` :`self` (`GameplayStatics.GetPlayerCameraManager` 0) :`FromAlpha` 1.0 :`Duration` 1.0)
  (`AudioComponent.Play` (`/Game/Pipes/Blueprints/BP_WidgerTitle.info_message` _bp_widgetfinal) 0.0)
  (bind _asfinal (cast `/Game/Pipes/Menu/Final` _returnvalue))
  (set `/Game/Pipes/Menu/Final.Text` "Вы победили трубы" _asfinal)
  (`/Game/Pipes/Menu/Final.set color` _asfinal true)
  (`Widget.SetVisibility` _returnvalue "Visible")
  (`KismetSystemLibrary.Delay` 5.0)
  (`GameplayStatics.OpenLevel` "StartMap"))

(fn `UserConstructionScript`)